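; BP_Door is a door actor that unlocks when every switch in its SwitchMaster array is pressed.
; Tick runs a DoOnce that assumes IsOpen is true, then clears it and resets the DoOnce if any switch's IsButtonPressed is false.
; Once all are pressed, the check stops repeating and a door-opening message prints; the graph contains no door movement.
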(event EventTick
  (params (DeltaSeconds :type Float%20%28single-precision%29))
  (Utilities|FlowControl|DoOnce false :!label _label
    (:Completed
      (Variables|Default|SetisOpen true)
      ;[0.15 0.15 0.15 0.5] For each switch object in the array, test if their varient of "isButtonPressed" is set to true. If not, set "IsOpen " to false and redo the sequence.
      (for _array_element (Variables|Default|GetSwitchMaster)
        (if (not (Variables|/Game/MyContent/MyBlueprints/BP_Switch.BP_Switch_C|GetIsButtonPressed _array_element))
          (Variables|Default|SetisOpen false)
          (goto _label Reset)))
      ;[0.15 0.15 0.15 0.5] ..If all are true, proceed to open the gate.
      (if (Variables|Default|GetisOpen)
        (Development|PrintString "\"You hear a door opening\"")))))

(fn ConstructionScript)